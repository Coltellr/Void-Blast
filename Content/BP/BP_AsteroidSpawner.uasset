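; Asteroid spawner actor that computes the visible play-area bounds for spawning; no spawning logic is present yet.
; One second after BeginPlay, it deprojects the viewport's top-left and bottom-right corners through player 0's controller.
; It intersects those rays with a horizontal plane to set the min and max X/Y spawn variables, so bounds follow the camera view and screen size at that moment.
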(event `self.ReceiveBeginPlay`
  (bind _returnvalue (`GameplayStatics.GetPlayerController` 0))
  (bind (_sizex _sizey) (`PlayerController.GetViewportSize` _returnvalue))
  (bind (_worldlocation _worlddirection) (`PlayerController.DeprojectScreenPositionToWorld` _returnvalue 0.0 0.0))
  (bind (_worldlocation_2 _worlddirection_2) (`PlayerController.DeprojectScreenPositionToWorld` _returnvalue (`KismetMathLibrary.Conv_IntToDouble` _sizex) (`KismetMathLibrary.Conv_IntToDouble` _sizey)))
  (bind (_t _intersection) (`KismetMathLibrary.LinePlaneIntersection` _worldlocation (+ _worldlocation (* _worlddirection (10000.0 10000.0 10000.0))) (make `Plane` 0.0 0.0 0.0 1.0)))
  (bind (_t_2 _intersection_2) (`KismetMathLibrary.LinePlaneIntersection` _worldlocation_2 (+ _worldlocation_2 (* _worlddirection_2 (10000.0 10000.0 10000.0))) (make `Plane` 0.0 0.0 0.0 1.0)))
  (`KismetSystemLibrary.Delay` 1.0)
  (set `self.SpawnMaxX` (.x _intersection))
  (set `self.SpawnMinY` (.y _intersection))
  (set `self.SpawnMinX` (.x _intersection_2))
  (set `self.SpawnMaxY` (.y _intersection_2)))

(fn `UserConstructionScript`)