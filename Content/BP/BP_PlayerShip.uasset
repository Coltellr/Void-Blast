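; Player ship Blueprint for a space shooter, handling screen-edge limits and visual and audio feedback.
; On BeginPlay, after a short delay, it deprojects opposite viewport corners onto a horizontal plane to set padded min/max X and Y bounds.
; Animation events swap Paper2D flipbooks for shooting and boost, with a shot sound.
; Death plays an explosion and sound, fades the camera, destroys the actor and calls GameOver on the game mode.
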(event `self.ReceiveBeginPlay`
  (bind _returnvalue (`GameplayStatics.GetPlayerController` 0))
  (bind _paddingship (`self.PaddingShip`))
  (bind (_sizex _sizey) (`PlayerController.GetViewportSize` _returnvalue))
  (bind (_worldlocation _worlddirection) (`PlayerController.DeprojectScreenPositionToWorld` _returnvalue 0.0 0.0))
  (bind (_worldlocation_2 _worlddirection_2) (`PlayerController.DeprojectScreenPositionToWorld` _returnvalue (`KismetMathLibrary.Conv_IntToDouble` _sizex) (`KismetMathLibrary.Conv_IntToDouble` _sizey)))
  (bind (_t _intersection) (`KismetMathLibrary.LinePlaneIntersection` _worldlocation (+ _worldlocation (* _worlddirection (10000.0 10000.0 10000.0))) (make `Plane` 0.0 0.0 0.0 1.0)))
  (bind (_t_2 _intersection_2) (`KismetMathLibrary.LinePlaneIntersection` _worldlocation_2 (+ _worldlocation_2 (* _worlddirection_2 (10000.0 10000.0 10000.0))) (make `Plane` 0.0 0.0 0.0 1.0)))
  (`KismetSystemLibrary.Delay` 0.2)
  (set `self.MaxX` (- (.x _intersection) _paddingship))
  (set `self.MinY` (+ (.y _intersection) _paddingship))
  (set `self.MinX` (+ (.x _intersection_2) _paddingship))
  (set `self.MaxY` (- (.y _intersection_2) _paddingship)))

(event `self.OnPlayShootAnim`
  (`|ExecutionSequence`
    (:`then_0`
      (`PaperFlipbookComponent.SetFlipbook` (`self.PaperFlipbook`) "/Game/UI/Textures/SpaceShip/FB_Ship_Shoot.FB_Ship_Shoot")
      (`KismetSystemLibrary.Delay` 0.15)
      (`PaperFlipbookComponent.SetFlipbook` (`self.PaperFlipbook`) "/Game/UI/Textures/SpaceShip/FB_Ship_Idle.FB_Ship_Idle"))
    (:`then_1`
      (`GameplayStatics.PlaySound2D` "/Game/UI/Sounds/SC_ShootSound.SC_ShootSound" 1.0 1.0 0.0 null null))))

(event `self.OnPlayDeathAnim`
  (`PaperFlipbookComponent.SetFlipbook` (`self.PaperFlipbook`) "/Game/UI/Textures/SpaceShip/FB_Ship_Explosion.FB_Ship_Explosion")
  (`GameplayStatics.PlaySound2D` "/Game/UI/Sounds/SC_DeathSound.SC_DeathSound" 1.0 1.0 0.0 null null)
  (`KismetSystemLibrary.Delay` 0.5)
  (`PlayerCameraManager.StartCameraFade` :`self` (`GameplayStatics.GetPlayerCameraManager` 0) :`ToAlpha` 1.0 :`Duration` 1.0 :`bHoldWhenFinished` true)
  (`KismetSystemLibrary.Delay` 1.1)
  (`self.K2_DestroyActor`)
  (bind _asspace_shooter_game_mode_base (cast `SpaceShooterGameModeBase` (`GameplayStatics.GetGameMode`)))
  (`SpaceShooterGameModeBase.GameOver` _asspace_shooter_game_mode_base))

(event `self.OnPlayBoostAnim`
  (`PaperFlipbookComponent.SetFlipbook` (`self.PaperFlipbook`) "/Game/UI/Textures/SpaceShip/FB_Ship_Boost.FB_Ship_Boost"))

(event `self.OnStopBoostAnim`
  (`PaperFlipbookComponent.SetFlipbook` (`self.PaperFlipbook`) "/Game/UI/Textures/SpaceShip/FB_Ship_Idle.FB_Ship_Idle"))

(fn `UserConstructionScript`)